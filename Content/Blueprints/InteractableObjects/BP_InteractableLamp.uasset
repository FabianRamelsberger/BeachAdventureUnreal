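; BP_InteractableLamp is an interactable lamp that the player toggles on and off through its Interaction event.
; BeginPlay creates a dynamic material instance from the lamp's mesh material.
; Each interaction flips IsLightOn, shows or hides the top and bottom lights, and sets the material's Emissive parameter to 1 or 0 to match.
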(event EventBeginPlay
  ;[0.15 0.15 0.15 0.5] Create Dynamic Material Instance
  (bind _returnvalue (Rendering|Material|CreateDynamicMaterialInstance (Variables|Default|GetObject) 0 0 "None" :!class /Script/Engine.PrimitiveComponent))
  (Variables|Default|SetLampMaterialInstance _returnvalue))

(event EventInteraction
  (bind _lampmaterialinstance (Variables|Default|GetLampMaterialInstance))
  ;[0.15 0.15 0.15 0.5] Sets the light on
  (if (Variables|Default|GetisLightOn)
    (Variables|Default|SetisLightOn false)
    (else
      (Variables|Default|SetisLightOn true)))
  (Rendering|SetVisibility (Variables|Default|GetTopLight) (Variables|Default|GetisLightOn) false)
  (if (Variables|Default|GetisLightOn)
    (Rendering|Material|SetScalarParameterValue _lampmaterialinstance "Emissive" 1.0 :!class /Script/Engine.MaterialInstanceDynamic)
    (else
      (Rendering|Material|SetScalarParameterValue _lampmaterialinstance "Emissive" 0.0 :!class /Script/Engine.MaterialInstanceDynamic))))

(fn ConstructionScript
  (|CallParentFunction))