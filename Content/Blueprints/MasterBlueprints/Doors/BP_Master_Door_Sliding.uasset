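; Master sliding door Blueprint that toggles a door mesh open and closed when its Interaction event fires.
; Interaction ignores input while the door moves, records its current relative location and flips the sign of the Y slide distance based on the open state.
; A Timeline then lerps the door along local Y and clears the moving flag when finished.
; The construction script pre-offsets doors flagged as open at start.
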(event Custom|SlideDoor
  (bind _slidingdoororigin (Variables|Default|GetSlidingDoorOrigin))
  (bind (_x _y _z) (Math|Vector|BreakVector _slidingdoororigin))
  ;[0.15 0.15 0.15 0.5] Slide Door with Timeline
  (bind _door_open_track (Timeline|Timeline PlayFromStart)
    (:Update
      (Transformation|SetRelativeLocation (Variables|Default|GetObject) (Math|Vector|Lerp(Vector) _slidingdoororigin (Math|Vector|MakeVector _x (+ _y (Variables|Default|GetSlidingY)) _z) _door_open_track) false false))
    (:Finished
      (Variables|Default|SetIsDoorMoving false))))

(event EventBeginPlay
  (|CallParentFunction) ; This node is disabled and will not be called.\nDrag off pins to build functionality.
)

(event EventInteraction
  ;[0.15 0.15 0.15 0.5] Interaction Door open/close
  (if (not (Variables|Default|GetIsDoorMoving))
    (Variables|Default|SetIsDoorMoving true)
    (Variables|Default|SetSlidingDoorOrigin (Variables|/Script/Engine.SceneComponent|GetRelativeLocation (Variables|Default|GetObject)))
    (if (Variables|Default|GetIsDoorOpen)
      (Variables|Default|SetIsDoorOpen false)
      (Variables|Default|SetSlidingY (* (Variables|Default|GetDoorSlidingY) -1.0))
      (else
        (Variables|Default|SetIsDoorOpen true)
        (Variables|Default|SetSlidingY (Variables|Default|GetDoorSlidingY))))
    (CallFunction|SlideDoor)))

(fn ConstructionScript
  (bind _object (Variables|Default|GetObject))
  (bind _relativelocation (Variables|/Script/Engine.SceneComponent|GetRelativeLocation _object))
  ;[0.15 0.15 0.15 0.5] Slide Door Open/Close at Start
  (if (Variables|Default|GetIsDoorOpen)
    (Transformation|SetRelativeLocation (Variables|Default|GetObject) (Math|Vector|MakeVector (.x _relativelocation) (+ (.y _relativelocation) (Variables|Default|GetDoorSlidingY)) (.z _relativelocation)) false false)))