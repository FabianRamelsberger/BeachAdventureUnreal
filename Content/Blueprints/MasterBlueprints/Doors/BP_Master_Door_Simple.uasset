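; Master Blueprint for a simple hinged door that swings open or closed when its Interaction event fires.
; The construction script offsets the door mesh by a quarter turn when IsDoorOpen is set, for doors that start open.
; Interaction ignores calls while moving, infers the swing direction from whether relative yaw is near zero, then drives a timeline that lerps the rotation from its current value.
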(event Custom|RotateDoor
  (bind _doororigin (Variables|Default|GetDoorOrigin))
  (bind (_roll _pitch _yaw) (Math|Rotator|BreakRotator _doororigin))
  ;[0.15 0.15 0.15 0.5] Rotate Door with Timeline
  (bind _door_open_track (Timeline|Timeline PlayFromStart)
    (:Update
      (Transformation|SetRelativeRotation (Variables|Default|GetObject) (Math|Rotator|Lerp(Rotator) _doororigin (Math|Rotator|MakeRotator _roll _pitch (+ _yaw (Variables|Default|GetDoorRotationYaw))) _door_open_track) false false))
    (:Finished
      (Variables|Default|SetIsDoorMoving false))))

(event EventBeginPlay
  (|CallParentFunction) ; This node is disabled and will not be called.\nDrag off pins to build functionality.
)

(event EventInteraction
  (bind _object (Variables|Default|GetObject))
  (bind _relativerotation (Variables|/Script/Engine.SceneComponent|GetRelativeRotation _object))
  ;[0.15 0.15 0.15 0.5] Interaction Door open/close
  (if (not (Variables|Default|GetIsDoorMoving))
    (Variables|Default|SetIsDoorMoving true)
    (Variables|Default|SetDoorOrigin _relativerotation)
    (if (Math|Float|NearlyEqual(Float) (.Yaw (Math|Rotator|BreakRotator _relativerotation)) 0.0 1.0)
      (Variables|Default|SetDoorRotationYaw -9e+01)
      (else
        (Variables|Default|SetDoorRotationYaw 9e+01)))
    (CallFunction|RotateDoor)))

(fn ConstructionScript
  (bind _object (Variables|Default|GetObject))
  (bind _relativerotation (Variables|/Script/Engine.SceneComponent|GetRelativeRotation _object))
  (bind (_roll _pitch _yaw) (Math|Rotator|BreakRotator _relativerotation))
  ;[0.15 0.15 0.15 0.5] Open / Close Door at Start
  (|CallParentFunction)
  (if (Variables|Default|GetIsDoorOpen)
    (Transformation|SetRelativeRotation (Variables|Default|GetObject) (Math|Rotator|MakeRotator _roll _pitch (+ _yaw -9e+01)) false false)))