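; Master Blueprint for inspectable objects that fly to the camera when interacted with, can be rotated, then return.
; Interaction disables movement, hides the HUD, re-centers the mesh and runs a timeline lerp to a point before the camera.
; Axis inputs rotate the actor, using camera-yaw quadrants to blend roll and pitch for view-relative tilting.
; Pressing Interact lerps it back, then restores HUD, movement and the game controller's inspection state.
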(event EventBeginPlay
  ;[0.15 0.15 0.15 0.5] Init Game Controller
  (bind _outactors (Actor|GetAllActorsOfClass "/Game/FirstPerson/BP_GameController.BP_GameController_C"))
  (Variables|Default|SetGameControllerInstance (Utilities|Array|Get(acopy) _outactors)))

(event EventInteraction
  (bind _gamecontrollerinstance (Variables|Default|GetGameControllerInstance))
  ;[0.15 0.15 0.15 0.5] MoveToCenterOfScreeenDisableInteraction
  (if (not (Variables|/Game/FirstPerson/BP_GameController.BP_GameController_C|GetIsInspection _gamecontrollerinstance))
    (Variables|/Game/FirstPerson/BP_GameController.BP_GameController_C|SetStopTrace _gamecontrollerinstance false)
    (|DisableMovementAndHideUI)
    (Variables|Default|SetObjectOriginRotator (Transformation|GetActorRotation))
    (Variables|Default|SetObjectOriginLocation (Transformation|GetActorLocation))
    (bind _movementtrack (Timeline|Movement PlayFromStart)
      (:Update
        (|UpdateMovementToCenterLocation _movementtrack))
      (:Finished
        (Variables|/Game/FirstPerson/BP_GameController.BP_GameController_C|SetIsInspection (Variables|Default|GetGameControllerInstance) true)
        (Input|EnableInput (Game|GetPlayerController 0))))))

(event Input|ActionEvents|InputActionInteract
  (params (Key :type Key%20Structure :default "None"))
  (bind _gamecontrollerinstance (Variables|Default|GetGameControllerInstance))
  ;[0.15 0.15 0.15 0.5] MoveObjectBack
  (:Pressed
    (Transformation|SetRelativeLocation (Variables|Default|GetInspectionObject) (Variables|Default|GetOriginRelativeLocation) false false)
    (Variables|/Script/Engine.SkeletalMeshComponent|SetbNoSkeletonUpdate (Variables|/Game/FirstPerson/BP_GameController.BP_GameController_C|GetGamePawnMeshRef (Variables|Default|GetGameControllerInstance)) false)
    (Input|DisableInput (Game|GetPlayerController 0))
    (Variables|Default|SetInspectionLocatoin (Transformation|GetActorLocation))
    (bind _movementbacktrack (Timeline|BackToOriginTimeLine PlayFromStart)
      (:Update
        (Transformation|SetActorLocationAndRotation (Math|Vector|Lerp(Vector) (Variables|Default|GetInspectionLocatoin) (Variables|Default|GetObjectOriginLocation) _movementbacktrack) (Variables|Default|GetObjectOriginRotator)))
      (:Finished
        (Variables|/Game/FirstPerson/BP_GameController.BP_GameController_C|SetIsInspection _gamecontrollerinstance false)
        (Widget|SetVisibility (Variables|Default|GetHudInstance) "Visible")
        (CallFunction|EnableMovement)
        (Variables|/Game/FirstPerson/BP_GameController.BP_GameController_C|SetStopTrace _gamecontrollerinstance false)))))

(event Input|AxisEvents|InputAxisRotate_Object_X
  (params (AxisValue :type Float%20%28single-precision%29))
  ;[0.15 0.15 0.15 0.5] Rotate Around X Axis
  (Class|Actor|AddActorWorldRotation (Math|Rotator|MakeRotator 0.0 0.0 (* AxisValue -1.0))))

(event Input|AxisEvents|InputAxisRotate_Object_Y
  (params (AxisValue :type Float%20%28single-precision%29))
  ;[0.15 0.15 0.15 0.5] Rotate Objet with Mouse Input
  (|SetQuadrant
    (:OutputPin
      (Variables|Default|SetRotationFactorX (|RotateFactorX))
      (Variables|Default|SetRotationFactorY (|RotateFactorY))
      (Class|Actor|AddActorWorldRotation (Math|Rotator|MakeRotator (* AxisValue (Variables|Default|GetRotationFactorX)) (* AxisValue (Variables|Default|GetRotationFactorY)) 0.0)))))

(fn ConstructionScript
  (|CallParentFunction))