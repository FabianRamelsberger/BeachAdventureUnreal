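; Master Blueprint for inspectable objects that float before the camera for rotation and can hold a hidden clue.
; Interaction pauses player tracing and hides the HUD, using a temporary static mesh copy for physics objects.
; Mouse rotation follows camera-yaw quadrants, while a looping timer trace detects sustained focus on the clue.
; Found clues turn toward the camera and shrink into the player, then PutBack timelines the object home and restores state.
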(event Custom|SetupStaticCopy
  ;[0.15 0.15 0.15 0.5] Setup a static copy for gravity
  (bind _returnvalue (AddComponent|AddStaticMeshComponent false))
  (bind _output_get (Variables|Setup|SetObjectCopy _returnvalue))
  (Components|StaticMesh|SetStaticMesh _output_get (Variables|/Script/Engine.StaticMeshComponent|GetStaticMesh (Variables|Default|GetObject)))
  (Collision|SetCollisionResponsetoChannel (Variables|Setup|GetObjectCopy) "ECC_Pawn" "ECR_Overlap")
  (bind _output_get_2 (Variables|Default|SetInspectionObject (Variables|Setup|GetObjectCopy)))
  (Physics|SetSimulatePhysics _output_get_2 false))

(event Custom|BackToPhisicsObject
  (bind _object (Variables|Default|GetObject))
  ;[0.15 0.15 0.15 0.5] GetObjectBackToPhysicsObject
  (Rendering|SetVisibility (Variables|Default|GetObject) true false)
  (Collision|SetCollisionResponsetoChannel _object "ECC_Pawn" "ECR_Block")
  (Physics|SetSimulatePhysics _object true)
  (Components|DestroyComponent (Variables|Setup|GetObjectCopy)))

(event Custom|TakeClueAnimation
  (bind _returnvalue (Game|Player|GetPlayerPawn 0))
  (bind _clue (Variables|Default|GetClue))
  (bind _returnvalue_2 (Transformation|GetActorLocation _returnvalue))
  ;[0.15 0.15 0.15 0.5] TakeClueAnimation
  (Variables|Default|SetClueLocation (Transformation|GetWorldLocation _clue))
  (Variables|Default|SetClueScale (Transformation|GetWorldScale _clue))
  (bind _scaling (Timeline|PutBackTimeline PlayFromStart)
    (:Update
      (Transformation|SetWorldScale3D (Variables|Default|GetClue) (Math|Vector|Lerp(Vector) (Variables|Default|GetClueScale) "0, 0, 0" _scaling))
      (Transformation|SetWorldLocation (Variables|Default|GetClue) (Math|Vector|Lerp(Vector) (Variables|Default|GetClueLocation) (Math|Vector|MakeVector (.x _returnvalue_2) (.y _returnvalue_2) (- (.z _returnvalue_2) 6e+01)) _scaling) false false))))

(event Custom|PutBack
  (bind _gamecontrollerinstance (Variables|Default|GetGameControllerInstance))
  ;[0.15 0.15 0.15 0.5] MoveObjectBack
  (Transformation|SetRelativeLocation (Variables|Default|GetInspectionObject) (Variables|Default|GetOriginRelativeLocation) false false)
  (Variables|/Script/Engine.SkeletalMeshComponent|SetbNoSkeletonUpdate (Variables|/Game/FirstPerson/BP_GameController.BP_GameController_C|GetGamePawnMeshRef (Variables|Default|GetGameControllerInstance)) false)
  (Input|DisableInput (Game|GetPlayerController 0))
  (Variables|Default|SetInspectionLocatoin (Transformation|GetActorLocation))
  (bind _movementbacktrack (Timeline|BackToOriginTimeLine PlayFromStart)
    (:Update
      (Transformation|SetActorLocationAndRotation (Math|Vector|Lerp(Vector) (Variables|Default|GetInspectionLocatoin) (Variables|Default|GetObjectOriginLocation) _movementbacktrack) (Variables|Rotation|GetObjectOriginRotator)))
    (:Finished
      (Variables|/Game/FirstPerson/BP_GameController.BP_GameController_C|SetIsInspection _gamecontrollerinstance false)
      (Widget|SetVisibility (Variables|Default|GetHudInstance) "Visible")
      (CallFunction|EnableMovement)
      (Variables|/Game/FirstPerson/BP_GameController.BP_GameController_C|SetStopTrace _gamecontrollerinstance false)
      (if (Variables|Setup|GetIsSimulatingPhysics)
        (CallFunction|BacktoPhisicsObject)
        (else
          (Collision|SetCollisionResponsetoChannel (Variables|Default|GetObject) "ECC_Pawn" "ECR_Block"))))))

(event EventBeginPlay
  ;[0.15 0.15 0.15 0.5] Init Game Controller
  (bind _outactors (Actor|GetAllActorsOfClass "/Game/FirstPerson/BP_GameController.BP_GameController_C"))
  (Variables|Default|SetGameControllerInstance (Utilities|Array|Get(acopy) _outactors)))

(event EventInteraction
  (bind _gamecontrollerinstance (Variables|Default|GetGameControllerInstance))
  (bind _object (Variables|Default|GetObject))
  ;[0.15 0.15 0.15 0.5] MoveToCenterOfScreeenDisableInteraction
  (if (not (Variables|/Game/FirstPerson/BP_GameController.BP_GameController_C|GetIsInspection _gamecontrollerinstance))
    (Variables|/Game/FirstPerson/BP_GameController.BP_GameController_C|SetStopTrace _gamecontrollerinstance true)
    (CallFunction|DisableMovement)
    (if (Variables|Setup|GetIsSimulatingPhysics)
      (Utilities|FlowControl|Sequence
        (:then_0
          (CallFunction|SetupStaticCopy))
        (:then_1
          (if (Variables|Default|GetIsClueTaken) :!label _label
            _
            (else
              (Utilities|Time|SetTimerbyFunctionName 0 "TraceForClue" 0.01 true)))
          (|DisableMovementAndHideUI)
          ;;[0.15 0.15 0.15 0.5] Save origin rotation and location depending on simulation phisics enabled
          (if (Variables|Setup|GetIsSimulatingPhysics)
            (Variables|Rotation|SetObjectOriginRotator (Transformation|GetWorldRotation _object))
            (Variables|Default|SetObjectOriginLocation (Transformation|GetWorldLocation _object))
            ;;[0.15 0.15 0.15 0.5] MoveToLocationAndEnableInput
            (bind _movementtrack (Timeline|Movement PlayFromStart)
              (:Update
                (|UpdateMovementToCenterLocation _movementtrack))
              (:Finished
                (Variables|/Game/FirstPerson/BP_GameController.BP_GameController_C|SetIsInspection (Variables|Default|GetGameControllerInstance) true)
                (Input|EnableInput (Game|GetPlayerController 0))))
            (else
              (Variables|Rotation|SetObjectOriginRotator (Transformation|GetActorRotation))
              (Variables|Default|SetObjectOriginLocation (Transformation|GetActorLocation))
              (Timeline|Movement PlayFromStart)))))
      (else
        ;;[0.15 0.15 0.15 0.5] Set A Copy
        (Variables|Default|SetInspectionObject (Variables|Default|GetObject))
        (goto _label)))))

(event Input|ActionEvents|InputActionInteract
  (params (Key :type Key%20Structure :default "None"))
  (:Pressed
    (CallFunction|PutBack)))

(event Input|ActionEvents|InputActionInteract2
  (params (Key :type Key%20Structure :default "None"))
  (:Pressed
    (CallFunction|PutBack)))

(event Input|AxisEvents|InputAxisRotate_Object_X
  (params (AxisValue :type Float%20%28single-precision%29))
  ;[0.15 0.15 0.15 0.5] Rotate Around X Axis
  (Class|Actor|AddActorWorldRotation (Math|Rotator|MakeRotator 0.0 0.0 (* AxisValue -1.0))))

(event Input|AxisEvents|InputAxisRotate_Object_Y
  (params (AxisValue :type Float%20%28single-precision%29))
  ;[0.15 0.15 0.15 0.5] Rotate Objet with Mouse Input
  (|SetQuadrant
    (:OutputPin
      (Variables|Rotation|SetRotationFactorX (|RotateFactorX))
      (Variables|Rotation|SetRotationFactorY (|RotateFactorY))
      (Class|Actor|AddActorWorldRotation (Math|Rotator|MakeRotator (* AxisValue (Variables|Rotation|GetRotationFactorX)) (* AxisValue (Variables|Rotation|GetRotationFactorY)) 0.0)))))

(fn ConstructionScript
  (|CallParentFunction)
  (Physics|SetSimulatePhysics (Variables|Default|GetObject) (Variables|Setup|GetIsSimulatingPhysics)))

(fn TraceforClue
  (bind _returnvalue (Game|GetPlayerCameraManager 0))
  (bind _returnvalue_2 (Camera|GetCameraLocation _returnvalue))
  (bind _outhit (Collision|LineTraceByChannel _returnvalue_2 (+ _returnvalue_2 (* (Transformation|GetActorForwardVector _returnvalue) 3e+02)) "TraceTypeQuery1" false 0 "None" false))
  (if (.bBlockingHit (Collision|BreakHitResult _outhit))
    (if (or (== (Variables|Default|GetClueTrigger) (.HitComponent (Collision|BreakHitResult _outhit))) (== (.HitComponent (Collision|BreakHitResult _outhit)) (Variables|Default|GetClue)))
      (bind _output_get (Variables|Default|SetClueFoundTimer (+ (Variables|Default|GetClueFoundTimer) 1)))
      (if (> _output_get (Variables|Setup|GetInspectTime))
        (Input|DisableInput (Game|GetPlayerController 0))
        (Utilities|Time|ClearTimerbyFunctionName 0 "TraceForClue")
        (CallFunction|ClueFound))
      (else
        (Variables|Default|SetClueFoundTimer 0)))))

(fn ClueFound
  (Utilities|Time|SetTimerbyFunctionName 0 "StartClueAnimation" 0.5))

(fn StartClueAnimation
  (Utilities|Time|SetTimerbyFunctionName 0 "RotateObjectTowardsCamera" 0.01 true))

(fn RotateObjectTowardsCamera
  (bind _returnvalue (Transformation|GetActorLocation))
  (bind _returnvalue_2 (Game|GetPlayerCameraManager 0))
  (bind _returnvalue_3 (Game|GetPlayerCameraManager 0))
  (bind _returnvalue_4 (Transformation|GetActorRotation))
  (bind _focusoncluerotation (Variables|Setup|GetFocusOnClueRotation))
  (bind _returnvalue_5 (Transformation|GetActorLocation _returnvalue_2))
  (bind _returnvalue_6 (Transformation|GetActorForwardVector _returnvalue_2))
  (bind _returnvalue_7 (Camera|GetCameraLocation _returnvalue_3))
  (bind (_roll _pitch _yaw) (Math|Rotator|BreakRotator _focusoncluerotation))
  (bind _returnvalue_8 (Math|Rotator|FindLookatRotation _returnvalue _returnvalue_7))
  (bind _returnvalue_9 (* _returnvalue_6 15.0))
  (bind (_roll_2 _pitch_2 _yaw_2) (Math|Rotator|BreakRotator _returnvalue_8))
  (bind _returnvalue_10 (+ _returnvalue_5 _returnvalue_9))
  (bind _returnvalue_11 (+ _yaw _yaw_2))
  (bind _returnvalue_12 (+ _roll _roll_2))
  (bind _returnvalue_13 (+ _pitch _pitch_2))
  (bind _returnvalue_14 (Math|Rotator|MakeRotator _returnvalue_12 _returnvalue_13 _returnvalue_11))
  (if (Utilities|Operators|EqualEqual _returnvalue_4 _returnvalue_14 1.0)
    (Utilities|IsValid (Variables|Default|GetClue)
      (:Is%20Valid
        (if (Utilities|Operators|EqualEqual (Transformation|GetWorldLocation (Variables|Default|GetClue)) _returnvalue_10 2.0)
          (CallFunction|TakeClue :!label _label)
          (else
            (Transformation|SetWorldLocation (Variables|Default|GetClue) (Math|Interpolation|VInterpTo (Transformation|GetWorldLocation (Variables|Default|GetClue)) _returnvalue_10 (Utilities|Time|GetWorldDeltaSeconds) 1.5) false false))))
      (:Is%20Not%20Valid
        (goto _label)))
    (else
      (Transformation|SetActorRotation (Math|Interpolation|RInterpTo _returnvalue_4 _returnvalue_14 (Utilities|Time|GetWorldDeltaSeconds) 4.0)))))

(fn TakeClue
  (Utilities|IsValid (Variables|Default|GetClue)
    (:Is%20Valid
      (CallFunction|TakeClueAnimation))
    (:Is%20Not%20Valid
      _))
  (Utilities|Time|ClearTimerbyFunctionName 0 "RotateObjectTowardsCamera")
  (Utilities|Time|SetTimerbyFunctionName 0 "PutBack" 1.0)
  (Variables|Default|SetIsClueTaken true))