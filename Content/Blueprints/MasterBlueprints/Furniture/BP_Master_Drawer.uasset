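; Master Blueprint for furniture with sliding drawers that open or close on interaction.
; Interaction slides the GameController's ActiveComponent along local Y via timeline, to DrawerDepth or zero depending on which half it sits in.
; The controller, fetched on BeginPlay with timer retry, has StopTrace set during movement.
; The construction script collects "Interactable"-tagged meshes and offsets them by OpenDrawers values for preset open positions.
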(event Custom|InitGameController
  ;[0.15 0.15 0.15 0.5] Init Game Controller
  (bind _outactors (Actor|GetAllActorsOfClass "/Game/FirstPerson/BP_GameController.BP_GameController_C"))
  (Utilities|IsValid (Utilities|Array|Get(acopy) _outactors)
    (:Is%20Valid
      (Variables|Default|SetGameControllerInstance (Utilities|Array|Get(acopy) _outactors)))
    (:Is%20Not%20Valid
      (Utilities|Time|SetTimerbyEvent (delegate Custom|InitGameController) 0.2))))

(event Custom|DrawerPushPull
  (bind _gamecontrollerinstance (Variables|Default|GetGameControllerInstance))
  (bind _activecomponent (Variables|/Game/FirstPerson/BP_GameController.BP_GameController_C|GetActiveComponent _gamecontrollerinstance))
  (bind _relativelocation (Variables|/Script/Engine.SceneComponent|GetRelativeLocation _activecomponent))
  ;[0.15 0.15 0.15 0.5] DrawerPush/Pull
  (Variables|Default|SetIsMoving true)
  (Variables|Default|SetDrawerOrigin (Variables|/Script/Engine.SceneComponent|GetRelativeLocation _activecomponent))
  (if (> (- (Variables|Default|GetDrawerDepth) (.y _relativelocation)) (.y _relativelocation))
    (Variables|Default|SetDrawerTarget (Variables|Default|GetDrawerDepth))
    (else
      (Variables|Default|SetDrawerTarget 0.0)))
  (CallFunction|MoveDrawer))

(event Custom|MoveDrawer
  (bind _drawerorigin (Variables|Default|GetDrawerOrigin))
  (bind (_x _y _z) (Math|Vector|BreakVector _drawerorigin))
  ;[0.15 0.15 0.15 0.5] MoveDrawer
  (bind _drawermovementtrack (Timeline|DrawerTimeLine PlayFromStart)
    (:Update
      (Transformation|SetRelativeLocation (Variables|/Game/FirstPerson/BP_GameController.BP_GameController_C|GetActiveComponent (Variables|Default|GetGameControllerInstance)) (Math|Vector|Lerp(Vector) _drawerorigin (Math|Vector|MakeVector _x (Variables|Default|GetDrawerTarget) _z) _drawermovementtrack) false false))
    (:Finished
      (Variables|Default|SetIsMoving false)
      (Variables|/Game/FirstPerson/BP_GameController.BP_GameController_C|SetStopTrace (Variables|Default|GetGameControllerInstance) false))))

(event EventBeginPlay
  ;[0.15 0.15 0.15 0.5] Init Game Controller
  (CallFunction|InitGameController))

(event EventInteraction
  ;[0.15 0.15 0.15 0.5] Interaction
  (if (not (Variables|Default|GetIsMoving))
    (Variables|/Game/FirstPerson/BP_GameController.BP_GameController_C|SetStopTrace (Variables|Default|GetGameControllerInstance) true)
    (CallFunction|DrawerPushPull)))

(fn ConstructionScript
  (bind _opendrawers (Variables|Default|GetOpenDrawers))
  (|CallParentFunction)
  (|GetAllDrawers
    (:Completed
      (if (Utilities|Array|IsValidIndex _opendrawers)
        (for (_array_element _array_index) _opendrawers
          (CallFunction|SetOpenDrawers _array_element _array_index))))))

(fn SetOpenDrawers
  (params (ArrayElement :type Float%20%28double-precision%29) (ArrayIndex :type Integer))
  (bind _drawers (Variables|Default|GetDrawers))
  (bind _output (Utilities|Array|Get(acopy) _drawers ArrayIndex))
  (bind _relativelocation (Variables|/Script/Engine.SceneComponent|GetRelativeLocation _output))
  (bind (_x _y _z) (Math|Vector|BreakVector _relativelocation))
  (Transformation|SetRelativeLocation _output (Math|Vector|MakeVector _x (+ ArrayElement _y) _z) false false))