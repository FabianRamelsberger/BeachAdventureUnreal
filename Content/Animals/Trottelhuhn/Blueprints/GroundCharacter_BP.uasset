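; Wandering animal character for the Trottelhuhn that repeatedly roams to random reachable points nearby.
; A Tick gate on IsMoving picks a point, then the Turn timeline rotates the capsule toward it before AIMoveTo runs.
; The animation Blueprint's State float is set high for travel and zeroed on arrival or failure.
; After a random pause, a looping timer ramps State up, then another pause releases the gate for the next move.
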(event Custom|IncreaseStateFloat
  (Math|Float|IncrementFloat (Variables|/Game/Animals/Trottelhuhn/Blueprints/GroundCharacter_Anim_BP.GroundCharacter_Anim_BP_C|GetState (Variables|Default|GetGroundCharacter%20BP))
    (:%20%20
      (if (not (< (Variables|/Game/Animals/Trottelhuhn/Blueprints/GroundCharacter_Anim_BP.GroundCharacter_Anim_BP_C|GetState (Variables|Default|GetGroundCharacter%20BP)) 1.5e+02))
        (Utilities|Time|ClearTimerbyFunctionName 0 "IncreaseStateFloat")
        (Utilities|FlowControl|Delay (Math|Random|RandomFloatinRange 3.0 7.0))
        (Variables|Default|SetisMoving? false)))))

(event EventBeginPlay
  (Components|Timeline|SetPlayRate (Variables|Character|GetMesh) 1.5)
  (bind _asground_character_anim_bp (Utilities|Casting|CastToGroundCharacter_Anim_BP (Components|SkeletalMesh|GetAnimInstance (Variables|Character|GetMesh))))
  (Variables|Default|SetGroundCharacter%20BP _asground_character_anim_bp))

(event EventTick
  (params (DeltaSeconds :type Float%20%28single-precision%29))
  (if (not (Variables|Default|GetisMoving?))
    (Variables|Default|SetisMoving? true)
    (Variables|Default|SetOriginRotation (Transformation|GetActorRotation))
    (Variables|Default|SetReachablePoint (.RandomLocation (AI|Navigation|GetRandomReachablePointinRadius (Transformation|GetActorLocation) 1.5e+03 0 0)))
    (bind _rotatehuhn (Timeline|Turn PlayFromStart)
      (:Update
        (Transformation|SetWorldRotation (Variables|Collision|GetCapsuleComponent) (Math|Rotator|Lerp(Rotator) (Variables|Default|GetOriginRotation) (Math|Rotator|FindLookatRotation (Transformation|GetActorLocation) (Variables|Default|GetReachablePoint)) _rotatehuhn) false false))
      (:Finished
        (Variables|/Game/Animals/Trottelhuhn/Blueprints/GroundCharacter_Anim_BP.GroundCharacter_Anim_BP_C|SetState (Variables|Default|GetGroundCharacter%20BP) 3e+02)
        (AI|AIMoveTo self (Variables|Default|GetReachablePoint) 0 5.0 false
          (:OnSuccess
            _)
          (:OnFail
            _))
        (Variables|/Game/Animals/Trottelhuhn/Blueprints/GroundCharacter_Anim_BP.GroundCharacter_Anim_BP_C|SetState (Variables|Default|GetGroundCharacter%20BP) 0.0)
        (Utilities|FlowControl|Delay (Math|Random|RandomFloatinRange 3.0 7.0))
        (Utilities|Time|SetTimerbyFunctionName 0 "IncreaseStateFloat" 0.01 true)))))

(fn ConstructionScript)