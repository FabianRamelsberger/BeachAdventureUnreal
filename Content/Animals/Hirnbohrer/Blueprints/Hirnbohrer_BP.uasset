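; Hirnbohrer animal Blueprint that wanders to random reachable points nearby, pausing at random intervals between moves.
; When not moving, Tick picks a point, a timeline turns the capsule toward it, then AIMoveTo walks there.
; The Anim BP's State float jumps high for movement and resets on arrival or failure.
; After a pause, a looping timer ramps State up to a threshold, then another delay re-arms the wander cycle.
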(event Custom|IncreaseStateFloat
  (Math|Float|IncrementFloat (Variables|/Game/Animals/Hirnbohrer/Blueprints/Hirnbohrer_Anim_BP.Hirnbohrer_Anim_BP_C|GetState (Variables|Default|GetAs%20Hirnbohrer%20Anim%20BP))
    (:%20%20
      (if (not (< (Variables|/Game/Animals/Hirnbohrer/Blueprints/Hirnbohrer_Anim_BP.Hirnbohrer_Anim_BP_C|GetState (Variables|Default|GetAs%20Hirnbohrer%20Anim%20BP)) 1.5e+02))
        (Utilities|Time|ClearTimerbyFunctionName 0 "IncreaseStateFloat")
        (Utilities|FlowControl|Delay (Math|Random|RandomFloatinRange 3.0 7.0))
        (Variables|Default|SetisMoving? false)))))

(event EventBeginPlay
  (Components|Timeline|SetPlayRate (Variables|Character|GetMesh) 1.5)
  (bind _ashirnbohrer_anim_bp (Utilities|Casting|CastToHirnbohrer_Anim_BP (Components|SkeletalMesh|GetAnimInstance (Variables|Character|GetMesh))))
  (Variables|Default|SetAs%20Hirnbohrer%20Anim%20BP _ashirnbohrer_anim_bp))

(event EventTick
  (params (DeltaSeconds :type Float%20%28single-precision%29))
  (if (not (Variables|Default|GetisMoving?))
    (Variables|Default|SetisMoving? true)
    (Variables|Default|SetOriginRotation (Transformation|GetActorRotation))
    (Variables|Default|SetReachablePoint (.RandomLocation (AI|Navigation|GetRandomReachablePointinRadius (Transformation|GetActorLocation) 1.5e+03 0 0)))
    (bind _rotatehirnbohrer (Timeline|Timeline_0 PlayFromStart)
      (:Update
        (Transformation|SetWorldRotation (Variables|Collision|GetCapsuleComponent) (Math|Rotator|Lerp(Rotator) (Variables|Default|GetOriginRotation) (Math|Rotator|FindLookatRotation (Transformation|GetActorLocation) (Variables|Default|GetReachablePoint)) _rotatehirnbohrer) false false))
      (:Finished
        (Variables|/Game/Animals/Hirnbohrer/Blueprints/Hirnbohrer_Anim_BP.Hirnbohrer_Anim_BP_C|SetState (Variables|Default|GetAs%20Hirnbohrer%20Anim%20BP) 3e+02)
        (AI|AIMoveTo self (Variables|Default|GetReachablePoint) 0 5.0 false
          (:OnSuccess
            _)
          (:OnFail
            _))
        (Variables|/Game/Animals/Hirnbohrer/Blueprints/Hirnbohrer_Anim_BP.Hirnbohrer_Anim_BP_C|SetState (Variables|Default|GetAs%20Hirnbohrer%20Anim%20BP) 0.0)
        (Utilities|FlowControl|Delay (Math|Random|RandomFloatinRange 3.0 7.0))
        (Utilities|Time|SetTimerbyFunctionName 0 "IncreaseStateFloat" 0.01 true)))))

(fn ConstructionScript)