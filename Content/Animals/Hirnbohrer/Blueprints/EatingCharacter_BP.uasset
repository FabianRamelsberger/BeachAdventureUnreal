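; EatingCharacter_BP is a wandering animal character in the Hirnbohrer folder that roams to random reachable points.
; When idle, Tick picks a point within a radius, and a Timeline turns the capsule toward it before AIMoveTo runs.
; It sets the anim Blueprint's State for movement, then resets it on success or failure and waits a random few seconds before roaming again.
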(event EventBeginPlay
  (Components|Timeline|SetPlayRate (Variables|Character|GetMesh) 1.5)
  (bind _aseating_character_anim_bp (Utilities|Casting|CastToEatingCharacter_Anim_BP (Components|SkeletalMesh|GetAnimInstance (Variables|Character|GetMesh))))
  (Variables|Default|SetEatingCharacter%20Character%20BP _aseating_character_anim_bp))

(event EventTick
  (params (DeltaSeconds :type Float%20%28single-precision%29))
  (if (not (Variables|Default|GetisMoving?))
    (Variables|Default|SetisMoving? true)
    (Variables|Default|SetOriginRotation (Transformation|GetActorRotation))
    (Variables|Default|SetReachablePoint (.RandomLocation (AI|Navigation|GetRandomReachablePointinRadius (Transformation|GetActorLocation) 1.5e+03 0 0)))
    (bind _rotatecharacter (Timeline|Timeline PlayFromStart)
      (:Update
        (Transformation|SetWorldRotation (Variables|Collision|GetCapsuleComponent) (Math|Rotator|Lerp(Rotator) (Variables|Default|GetOriginRotation) (Math|Rotator|FindLookatRotation (Transformation|GetActorLocation) (Variables|Default|GetReachablePoint)) _rotatecharacter) false false))
      (:Finished
        (Variables|/Game/Animals/Hirnbohrer/Blueprints/EatingCharacter_Anim_BP.EatingCharacter_Anim_BP_C|SetState (Variables|Default|GetEatingCharacter%20Character%20BP) 3e+02)
        (AI|AIMoveTo self (Variables|Default|GetReachablePoint) 0 5.0 false
          (:OnSuccess
            _)
          (:OnFail
            _))
        (Variables|/Game/Animals/Hirnbohrer/Blueprints/EatingCharacter_Anim_BP.EatingCharacter_Anim_BP_C|SetState (Variables|Default|GetEatingCharacter%20Character%20BP) 0.0)
        (Utilities|FlowControl|Delay (Math|Random|RandomFloatinRange 3.0 7.0))
        (Variables|Default|SetisMoving? false)))))

(fn ConstructionScript)